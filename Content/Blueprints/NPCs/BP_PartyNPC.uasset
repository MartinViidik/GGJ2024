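; Party guest NPC that roams near its spawn and accosts the player to demand a joke.
; Sphere overlap turns its eyes red via a dynamic material, starts a chase and enables a Tick distance check.
; Up close, it freezes the player, with timelines easing player rotation and camera FOV, then triggers TellMeAJoke and depletes jokes.
; It then heads for BP_ExitPoint while player control and FOV are restored; LeaveArea destroys it.
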(event `self.ReceiveBeginPlay`
  (set `self.OriginLocation` (`self.K2_GetActorLocation`))
  (`self.RoamLogic`)
  (bind _returnvalue (`PrimitiveComponent.CreateDynamicMaterialInstance` (`self.StaticMesh5`) 0 "/Game/Materials/M_EyeMaterial.M_EyeMaterial" "None"))
  (bind _output_get (set `self.EyeMaterial` _returnvalue))
  (`MaterialInstanceDynamic.SetVectorParameterValue` _output_get "EyeColor" (struct :`R` 1.0 :`G` 1.0 :`B` 1.0 :`A` 1.0)))

(event `RoamLogic`
  (bind (_randomlocation _returnvalue) (`NavigationSystemV1.K2_GetRandomReachablePointInRadius` (`self.OriginLocation`) 1024.0 null null))
  (if (`self.Leaving`)
    _
    (elif _returnvalue
      (`|AIMoveTo` self _randomlocation null 100.0
        (:`OnSuccess`
          (`KismetSystemLibrary.Delay` (+ (`KismetMathLibrary.RandomFloatInRange` 0.0 2.0) 4.0))
          (`self.RoamLogic`)))
      (else
        (`self.RoamLogic`)))))

(event `MoveToObject`
  (params (TargetActor :type "Actor Object Reference"))
  (`|AIMoveTo` self (`self.K2_GetActorLocation` TargetActor) TargetActor
    (:`OnSuccess`
      (`KismetSystemLibrary.Delay` 4.0)
      (`self.RoamLogic`))))

(event `self.SphereCollision.OnComponentBeginOverlap`
  (params (OverlappedComponent :type "PrimitiveComponent Object Reference") (OtherActor :type "Actor Object Reference") (OtherComp :type "PrimitiveComponent Object Reference") (OtherBodyIndex :type Integer) (bFromSweep :type Boolean) (SweepResult :type "HitResult Structure (by ref)"))
  (if (not (`self.Leaving`))
    (bind _asbp_third_person_character (cast `/Game/ThirdPerson/Blueprints/BP_ThirdPersonCharacter` OtherActor))
    (set `self.As BP Third Person Character` _asbp_third_person_character)
    (`self.MoveToObject` _asbp_third_person_character)
    (`MaterialInstanceDynamic.SetVectorParameterValue` (`self.EyeMaterial`) "EyeColor" (struct :`R` 100.0 :`A` 1.0))
    (`self.SetActorTickEnabled` true)))

(event `self.SphereCollision.OnComponentEndOverlap`
  (params (OverlappedComponent :type "PrimitiveComponent Object Reference") (OtherActor :type "Actor Object Reference") (OtherComp :type "PrimitiveComponent Object Reference") (OtherBodyIndex :type Integer))
  (if (not (`self.Leaving`))
    (cast `/Game/ThirdPerson/Blueprints/BP_ThirdPersonCharacter` OtherActor)
    (set `self.As BP Third Person Character` null)
    (`self.RoamLogic`)
    (`MaterialInstanceDynamic.SetVectorParameterValue` (`self.EyeMaterial`) "EyeColor" (struct :`R` 1.0 :`G` 1.0 :`B` 1.0 :`A` 1.0))
    (`self.SetActorTickEnabled` false)))

(event `self.ReceiveTick`
  (params (DeltaSeconds :type "Float (single-precision)"))
  (if (<= (`self.GetDistanceTo` (`self.As BP Third Person Character`) self) 200.0)
    (`self.SetActorTickEnabled` false)
    (`self.DemandAJoke`)))

(event `DemandAJoke`
  (`CharacterMovementComponent.SetMovementMode` (`Character.CharacterMovement` (`self.As BP Third Person Character`)) "MOVE_None" 0)
  (bind (_direction _newtrack_0) (`Timeline|Timeline`)
    (:`Update`
      (`self.K2_SetActorRotation` (`self.As BP Third Person Character`) (`KismetMathLibrary.RInterpTo` (`self.K2_GetActorRotation` (`self.As BP Third Person Character`)) (`KismetMathLibrary.Conv_VectorToRotator` (* (`self.K2_GetActorRotation`) -1.0)) _newtrack_0 1.0) false)
      (`CameraComponent.SetFieldOfView` (`/Game/ThirdPerson/Blueprints/BP_ThirdPersonCharacter.FollowCamera` (`self.As BP Third Person Character`)) (`KismetMathLibrary.FInterpTo` 90.0 60.0 _newtrack_0 1.0)))
    (:`Finished`
      (`KismetSystemLibrary.Delay` 1.0)
      (`/Game/ThirdPerson/Blueprints/BP_ThirdPersonCharacter.TellMeAJoke` (`self.As BP Third Person Character`))
      (`KismetSystemLibrary.Delay` 3.5)
      (set `self.Leaving` true)
      (`self.SetActorEnableCollision` (`self.As BP Third Person Character`) false)
      (set `CharacterMovementComponent.MaxWalkSpeed` 350.0 (`self.CharacterMovement`))
      (bind _returnvalue (`GameplayStatics.GetActorOfClass` "/Game/Blueprints/Misc/BP_ExitPoint.BP_ExitPoint_C"))
      (`self.MoveToObject` _returnvalue)
      (`self.ReturnToNormal`)
      (`/Game/Blueprints/Components/BPC_PlayerState.DepleteJokes` (`/Game/ThirdPerson/Blueprints/BP_ThirdPersonCharacter.BPC_PlayerState` (`self.As BP Third Person Character`)) 25.0))))

(event `ReturnToNormal`
  (`KismetSystemLibrary.Delay` 2.0)
  (bind (_direction _newtrack_0) (`Timeline|Timeline_0` :!via `PlayFromStart`)
    (:`Update`
      (`CameraComponent.SetFieldOfView` (`/Game/ThirdPerson/Blueprints/BP_ThirdPersonCharacter.FollowCamera` (`self.As BP Third Person Character`)) (`KismetMathLibrary.FInterpTo` 60.0 90.0 _newtrack_0 1.0)))
    (:`Finished`
      (`self.SetActorEnableCollision` (`self.As BP Third Person Character`) true)
      (`CharacterMovementComponent.SetMovementMode` (`Character.CharacterMovement` (`self.As BP Third Person Character`)) "MOVE_Walking" 0))))

(event `LeaveArea`
  (`self.K2_DestroyActor`))

(fn `UserConstructionScript`)