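; Player state component that tracks the food and jokes resources for the third-person character.
; A looping timer starts on BeginPlay, and DepleteFood lowers food by its depletion rate, signalling depletion and clearing the timer at zero.
; DepleteJokes subtracts a passed amount; both depletion events update fill bars through the character's UI reference.
; SetResource switches on resource type and adds to food, without refreshing the UI.
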(event `self.ReceiveBeginPlay`
  (bind _returnvalue (`KismetSystemLibrary.K2_SetTimerDelegate` (`|CreateDelegate` :!event `DepleteFood`) 1.0 true))
  (set `self.FoodTimer` _returnvalue)
  (bind _asbp_third_person_character (cast `/Game/ThirdPerson/Blueprints/BP_ThirdPersonCharacter` (`self.GetOwner`)))
  (set `self.As BP Third Person Character` _asbp_third_person_character))

(event `DepleteFood`
  (set `self.FoodValue` (- (`self.FoodValue`) (`self.FoodDepletionRate`)))
  (`/Game/Blueprints/UI/WBP_MainWidget.SetFoodFillAmount` (`/Game/ThirdPerson/Blueprints/BP_ThirdPersonCharacter.UIReference` (`self.As BP Third Person Character`)) (`self.FoodValue`))
  (if (<= (`self.FoodValue`) 0.0)
    (`self.ResourceDepleted` "NewEnumerator0")
    (`KismetSystemLibrary.K2_ClearAndInvalidateTimerHandle` (`self.FoodTimer`))))

(event `DepleteJokes`
  (params (NewParam :type "Float (double-precision)"))
  (bind _output_get (set `self.JokesValue` (- (`self.JokesValue`) NewParam)))
  (`/Game/Blueprints/UI/WBP_MainWidget.SetPartyFillAmount` (`/Game/ThirdPerson/Blueprints/BP_ThirdPersonCharacter.UIReference` (`self.As BP Third Person Character`)) _output_get))

(fn `SetResource`
  (params (Amount :type "Float (double-precision)") (ResourceType :type "/Game/Misc/ENUM_Resources Enum" :default "NewEnumerator0"))
  (switch `/Game/Misc/ENUM_Resources` ResourceType
    (:`NewEnumerator0`
      (set `self.FoodValue` (+ (`self.FoodValue`) Amount)))))