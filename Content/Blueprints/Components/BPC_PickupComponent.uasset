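; Actor component that lets its owner pick up resources from pickup points and deliver them.
; Capsule overlaps track the current BP_ResourcePickupPoint, from which Pickup spawns a resource and snaps it to the owner's "PickupPoint"-tagged component.
; Drop broadcasts ObjectDelivered with the item's replenish rate and resource type, calls AttractNPC on the target delivery point, then destroys the item.
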(event `self.ReceiveBeginPlay`
  (bind _output_get (set `self.Owner` (`self.GetOwner`)))
  (bind _returnvalue (`Actor.GetComponentByClass` _output_get "/Script/Engine.CapsuleComponent"))
  (add `PrimitiveComponent.OnComponentBeginOverlap` _returnvalue (`|CreateDelegate` :!event `StartOverlap`))
  (add `PrimitiveComponent.OnComponentEndOverlap` _returnvalue (`|CreateDelegate` :!event `StopOverlap`)))

(event `StartOverlap`
  (params (OverlappedComponent :type "PrimitiveComponent Object Reference") (OtherActor :type "Actor Object Reference") (OtherComp :type "PrimitiveComponent Object Reference") (OtherBodyIndex :type Integer) (bFromSweep :type Boolean) (SweepResult :type "HitResult Structure (by ref)"))
  (bind _asbp_resource_pickup_point (cast `/Game/Blueprints/Items/BP_ResourcePickupPoint` OtherActor))
  (set `self.As BP Resource Pickup Point` _asbp_resource_pickup_point))

(event `StopOverlap`
  (params (OverlappedComponent :type "PrimitiveComponent Object Reference") (OtherActor :type "Actor Object Reference") (OtherComp :type "PrimitiveComponent Object Reference") (OtherBodyIndex :type Integer))
  (set `self.As BP Resource Pickup Point` null))

(event `Pickup`
  (bind _returnvalue (`/Game/Blueprints/Items/BP_ResourcePickupPoint.SpawnResource` (`self.As BP Resource Pickup Point`)))
  (bind _output_get (set `self.PickedUpObject` _returnvalue))
  (`Actor.K2_AttachToComponent` _output_get (`|GetArrayItem` (`Actor.GetComponentsByTag` (`self.Owner`) "/Script/Engine.SceneComponent" "PickupPoint")) "None" "SnapToTarget" "SnapToTarget" "SnapToTarget" true)
  (set `self.As BP Resource Pickup Point` null))

(event `Drop`
  (bind _returnvalue (`Actor.GetComponentByClass` (`self.PickedUpObject`) "/Game/Blueprints/Components/BPC_PickupableComponent.BPC_PickupableComponent_C"))
  (`self.ObjectDelivered` (`/Game/Blueprints/Components/BPC_PickupableComponent.ReplenishRate` _returnvalue) (`/Game/Blueprints/Components/BPC_PickupableComponent.ResourceType` _returnvalue))
  (`/Game/Blueprints/Components/BPC_DeliveryPoint.AttractNPC` (`self.TargetDeliverPoint`))
  (`Actor.K2_DestroyActor` (`self.PickedUpObject`))
  (`KismetSystemLibrary.PrintString` "Delivered"))