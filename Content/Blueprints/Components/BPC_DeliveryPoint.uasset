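; Actor component that marks its owner as a delivery point for one target resource type.
; It binds to the owner's sphere overlaps and, on entry, finds the object carried through the overlapping actor's BPC_PickupComponent.
; That object's BPC_PickupableComponent gets ReadyToDeliver set according to whether its resource type matches.
; The flag clears when the last stored overlapping actor leaves; the delivery itself happens outside this component.
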(event `self.ReceiveBeginPlay`
  (bind _returnvalue (`Actor.GetComponentByClass` (`self.GetOwner`) "/Script/Engine.SphereComponent"))
  (add `PrimitiveComponent.OnComponentBeginOverlap` _returnvalue (`|CreateDelegate` :!event `OnBeginOverlap`))
  (add `PrimitiveComponent.OnComponentEndOverlap` _returnvalue (`|CreateDelegate` :!event `OnEndOverlap`)))

(event `OnBeginOverlap`
  (params (OverlappedComponent :type "PrimitiveComponent Object Reference") (OtherActor :type "Actor Object Reference") (OtherComp :type "PrimitiveComponent Object Reference") (OtherBodyIndex :type Integer) (bFromSweep :type Boolean) (SweepResult :type "HitResult Structure (by ref)"))
  (`self.CheckDelivery` OtherActor))

(event `OnEndOverlap`
  (params (OverlappedComponent :type "PrimitiveComponent Object Reference") (OtherActor :type "Actor Object Reference") (OtherComp :type "PrimitiveComponent Object Reference") (OtherBodyIndex :type Integer))
  (bind _pickupcomponent (`self.PickupComponent`))
  (if (== OtherActor (`self.TargetActor`))
    (`/Engine/EditorBlueprintResources/StandardMacros.IsValid` _pickupcomponent
      (:`Is Valid`
        (set `/Game/Blueprints/Components/BPC_PickupableComponent.ReadyToDeliver` false _pickupcomponent)))))

(fn `CheckDelivery`
  (params (TargetActor :type "Actor Object Reference"))
  (bind _returnvalue (`Actor.GetComponentByClass` TargetActor "/Game/Blueprints/Components/BPC_PickupComponent.BPC_PickupComponent_C"))
  (bind _returnvalue_2 (`Actor.GetComponentByClass` (`/Game/Blueprints/Components/BPC_PickupComponent.PickedUpObject` _returnvalue) "/Game/Blueprints/Components/BPC_PickupableComponent.BPC_PickupableComponent_C"))
  (set `self.TargetActor` TargetActor)
  (`/Engine/EditorBlueprintResources/StandardMacros.IsValid` _returnvalue
    (:`Is Valid`
      (`/Engine/EditorBlueprintResources/StandardMacros.IsValid` _returnvalue_2
        (:`Is Valid`
          (set `self.PickupComponent` _returnvalue_2)
          (set `/Game/Blueprints/Components/BPC_PickupableComponent.ReadyToDeliver` (`|EnumEquality` (`self.TargetResource`) (`/Game/Blueprints/Components/BPC_PickupableComponent.ResourceType` _returnvalue_2)) (`self.PickupComponent`)))))))

(fn `IsValidResource`
  (params (InResource :type "/Game/Misc/ENUM_Resources Enum" :default "NewEnumerator0"))
  (returns (IsValid :type Boolean))
  (return (`|EnumEquality` InResource (`self.TargetResource`))))